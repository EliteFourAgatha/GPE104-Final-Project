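; WinCondition is a level-exit trigger actor that advances the game when any actor begins overlapping it.
; On overlap it plays a magical portal sound at the world origin, then waits briefly before checking the current level name.
; A hardcoded chain of name checks opens the next level by name, running from Level1 through Level3 and ending at Credits.
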(event `self.ReceiveActorBeginOverlap`
  (params (OtherActor :type "Actor Object Reference"))
  (`GameplayStatics.PlaySoundAtLocation` "/Game/SFX/401324__alanmcki__magical-portal-open.401324__alanmcki__magical-portal-open" (0.0 0.0 0.0) (struct) 1.0 1.0 0.0 null null null)
  (`KismetSystemLibrary.Delay` 2.0)
  (bind _returnvalue (`GameplayStatics.GetCurrentLevelName` true))
  (if (`KismetStringLibrary.EqualEqual_StrStr` _returnvalue "Level1")
    (`GameplayStatics.OpenLevel` "Level2")
    (elif (`KismetStringLibrary.EqualEqual_StrStr` _returnvalue "Level2")
      (`GameplayStatics.OpenLevel` "Level3")
      (elif (`KismetStringLibrary.EqualEqual_StrStr` _returnvalue "Level3")
        (`GameplayStatics.OpenLevel` "Credits")))))

(fn `UserConstructionScript`)